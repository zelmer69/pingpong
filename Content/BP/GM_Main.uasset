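; Game mode for a multiplayer ball game that starts play once more than one player has joined.
; PostLogin spawns a B_Ball at the world origin when that player count is met, and the Goal event spawns another through the same SpawnBall function.
; ChoosePlayerStart assigns each player the PlayerStart matching their PlayerArray index.
; Ball yaw comes from an unscaled RandomFloat, so it varies by under one degree.
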(event EventBeginPlay)

(event EventTick
  (params (DeltaSeconds :type Float%20%28single-precision%29)))

(event EventPostLogin
  (params (NewPlayer :type Player%20Controller%20Object%20Reference))
  (Development|PrintString "New player has joined")
  (if (> (Utilities|Array|Length (Variables|/Script/Engine.GameStateBase|GetPlayerArray (Game|GetGameState))) 1)
    (Development|PrintString "Starting the game")
    (CallFunction|SpawnBall)
    (else
      (Development|PrintString "Waiting for second player"))))

(event EventGoal
  (params (PlayerID :type Integer))
  (CallFunction|SpawnBall))

(fn ConstructionScript)

(fn ChoosePlayerStart
  (params (Player :type Controller%20Object%20Reference))
  (bind _outactors (Actor|GetAllActorsOfClass "/Script/Engine.PlayerStart"))
  (return (Utilities|Array|Get(acopy) _outactors (Utilities|Array|FindItem (Variables|/Script/Engine.GameStateBase|GetPlayerArray (Game|GetGameState)) (Variables|/Script/Engine.Controller|GetPlayerState Player)))))

(fn SpawnBall
  (Game|SpawnActorfromClass "/Game/BP/B_Ball.B_Ball_C" (Math|Transform|MakeTransform "0, 0, 0" (Math|Rotator|MakeRotator 0.0 0.0 (Math|Random|RandomFloat))) "Undefined" 0 0))